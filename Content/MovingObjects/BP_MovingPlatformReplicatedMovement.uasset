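; Moving platform that rises above its start location and returns on a repeating cycle, driven by the server.
; BeginPlay stores the start location and, on authority only, starts a looping timer, presumably bound to MovePlatform.
; MovePlatform alternates playing and reversing a timeline that lerps the actor's height without sweep.
; The graph has no RPCs or replication logic; as the asset name indicates, clients rely on replicated movement.
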(event `self.ReceiveBeginPlay`
  (set `self.StartLocation` (`self.K2_GetActorLocation`))
  (`/Engine/EditorBlueprintResources/ActorMacros.Switch Has Authority`
    (:`Authority`
      (`KismetSystemLibrary.K2_SetTimerDelegate` (`|CreateDelegate` :!event `MovePlatform`) 2.5 true))))

(event `MovePlatform`
  (bind (_startlocation_x _startlocation_y _startlocation_z) (`KismetMathLibrary.BreakVector` (`self.StartLocation`)))
  (`/Engine/EditorBlueprintResources/StandardMacros.FlipFlop`
    (:`A`
      (bind (_direction _alpha) (`Timeline|TL_MovePlatform` :!label _label)
        (:`Update`
          (`self.K2_SetActorLocation` (`KismetMathLibrary.VLerp` (`self.StartLocation`) (`KismetMathLibrary.MakeVector` _startlocation_x _startlocation_y (+ _startlocation_z 220.0)) _alpha)))))
    (:`B`
      (goto _label :!via `Reverse`))))

(fn `UserConstructionScript`)