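; BP_Interactable is a one-way lever in the world that activates a linked actor when interacted with.
; Interact sets the replicated DidInteract flag, and its RepNotify carries out the visible response.
; The notify pitches the lever hinge over, calls ClientActivate on ActorToActivate and disables collision on Sphere1, with no reset path in the graph.
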(event `Interact`
  (set `self.bDidInteract` true))

(event `FlipLever`
  (bind _leverhinge (`self.LeverHinge`))
  (bind (_relativerotation_roll _relativerotation_pitch _relativerotation_yaw) (`KismetMathLibrary.BreakRotator` (`SceneComponent.RelativeRotation` _leverhinge)))
  (`SceneComponent.K2_SetRelativeRotation` _leverhinge (`KismetMathLibrary.MakeRotator` _relativerotation_roll (- _relativerotation_pitch -70.0) _relativerotation_yaw) false false))

(fn `OnRep_bDidInteract`
  (`self.FlipLever`)
  (`/Game/MovingObjects/BP_Activateable.ClientActivate` (`self.ActorToActivate`))
  (`PrimitiveComponent.SetCollisionEnabled` (`self.Sphere1`) "NoCollision"))

(fn `UserConstructionScript`)