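; BP_Activateable is a moving object whose Cube slides to a fixed relative position when activated.
; BeginPlay caches the Cube's starting relative location.
; ClientActivate plays the TL_MovePlatform timeline, which lerps the Cube from that start to the raised target without sweep and flags FinishedMove on completion.
; An unconnected branch that checks FinishedMove to replay or snap to the target never runs.
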(event `self.ReceiveBeginPlay`
  (set `self.Relative Location` (`SceneComponent.RelativeLocation` (`self.Cube`))))

(event `ClientActivate`
  (bind (_direction _alpha) (`Timeline|TL_MovePlatform`)
    (:`Update`
      (`SceneComponent.K2_SetRelativeLocation` (`self.Cube`) (`KismetMathLibrary.VLerp` (`self.Relative Location`) (0.0 0.0 90.0) _alpha) false false))
    (:`Finished`
      (set `self.bFinishedMove` true))))

(fn `UserConstructionScript`)