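; Moving platform actor that raises itself vertically from its starting location, driven by a timeline.
; BeginPlay caches the start location and slows the timeline's play rate, then only the authority waits briefly and calls ClientMovePlatform.
; That event plays the timeline, whose alpha interpolates the actor's location toward a fixed height offset, without sweep or teleport.
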(event `self.ReceiveBeginPlay`
  (set `self.StartLocation` (`self.K2_GetActorLocation`))
  (`TimelineComponent.SetPlayRate` (`self.TL_MovePlatform`) 0.7)
  (`/Engine/EditorBlueprintResources/ActorMacros.Switch Has Authority`
    (:`Authority`
      (`KismetSystemLibrary.Delay` 2.0)
      (`self.ClientMovePlatform`))))

(event `ClientMovePlatform`
  (bind (_startlocation_x _startlocation_y _startlocation_z) (`KismetMathLibrary.BreakVector` (`self.StartLocation`)))
  (bind (_direction _alpha) (`Timeline|TL_MovePlatform`)
    (:`Update`
      (`self.K2_SetActorLocation` (`KismetMathLibrary.VLerp` (`self.StartLocation`) (`KismetMathLibrary.MakeVector` _startlocation_x _startlocation_y (+ _startlocation_z 220.0)) _alpha)))))

(fn `UserConstructionScript`)