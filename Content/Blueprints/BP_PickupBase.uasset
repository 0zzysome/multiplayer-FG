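; Base pickup actor that bobs in place, reacts to the first-person character and respawns after a cooldown.
; A Timeline lerps the mesh's relative height at a rate set by the cycle speed.
; Collider overlap passes a DoOnce before the character cast, then calls OnPickedUp, hides the mesh and disables collision.
; A timer drives the respawn, which restores visibility and collision and resets the DoOnce.
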(event `self.ReceiveBeginPlay`
  ; Mesh bobbing up and down
  (`KismetSystemLibrary.Delay` 0.2)
  (`TimelineComponent.SetPlayRate` (`self.Timeline`) (/ 1.0 (`self.BobingCycleSpeed`)))
  (bind _output_get (set `self.Location` (`SceneComponent.RelativeLocation` (`self.PickupMesh`))))
  (bind (_direction _newtrack_1) (`Timeline|Timeline`)
    (:`Update`
      (`SceneComponent.K2_SetRelativeLocation` (`self.PickupMesh`) (`KismetMathLibrary.VLerp` _output_get (+ _output_get (0.0 0.0 20.0)) _newtrack_1) false false))))

(event `self.PickupCollider.OnComponentBeginOverlap`
  (params (OverlappedComponent :type "PrimitiveComponent Object Reference") (OtherActor :type "Actor Object Reference") (OtherComp :type "PrimitiveComponent Object Reference") (OtherBodyIndex :type Integer) (bFromSweep :type Boolean) (SweepResult :type "HitResult Structure (by ref)"))
  ; Pickup and respawn funtionality
  (`/Engine/EditorBlueprintResources/StandardMacros.DoOnce` false :!label _label
    (:`Completed`
      (bind _asbp_first_person_character (cast `/Game/FirstPerson/Blueprints/BP_FirstPersonCharacter` OtherActor))
      (`self.OnPickedUp` _asbp_first_person_character)
      (`SceneComponent.SetVisibility` (`self.PickupMesh`) false true)
      (`PrimitiveComponent.SetCollisionEnabled` (`self.PickupCollider`) "NoCollision")
      (`KismetSystemLibrary.K2_SetTimerDelegate` (`|CreateDelegate` :!event `Respawn pickup`) (`self.RespawnCooldown`)))))

(event `Respawn pickup`
  ; Pickup and respawn funtionality
  (`SceneComponent.SetVisibility` (`self.PickupMesh`) true true)
  (`PrimitiveComponent.SetCollisionEnabled` (`self.PickupCollider`) "QueryOnly")
  (goto _label :!via `Reset`))

(fn `UserConstructionScript`)