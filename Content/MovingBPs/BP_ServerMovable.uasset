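; BP_ServerMovable is an actor that swings its Pivot component when a linked Button is pressed.
; On BeginPlay it binds to the Button's Pressed dispatcher, or prints a warning if none is valid.
; A press calls Launch, which plays the TL_ServerRotation timeline from the start.
; Each update stores the timeline alpha and calls ClientUpdateLocation, which lerps the Pivot's relative pitch.
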(event `self.ReceiveBeginPlay`
  (bind _button (`self.Button`)
    (:`then`
      (add `/Game/MovingBPs/BP_InteractableBase.Pressed` _button (delegate `Pressed_Event`)))
    (:`else`
      (`KismetSystemLibrary.PrintString` "NO BUTTON FOUND"))))

(event `Pressed_Event`
  (`self.Launch`))

(event `Launch`
  (bind (_direction _alpha) (`Timeline|TL_ServerRotation` :!via `PlayFromStart`)
    (:`Update`
      (set `self.Alpha` _alpha)
      (`self.ClientUpdateLocation`))))

(event `ClientUpdateLocation`
  (`SceneComponent.K2_SetRelativeRotation` (`self.Pivot`) (`KismetMathLibrary.MakeRotator` 0.0 (`KismetMathLibrary.Lerp` 0.0 -100.0 (`self.Alpha`))) false false))

(fn `UserConstructionScript`)