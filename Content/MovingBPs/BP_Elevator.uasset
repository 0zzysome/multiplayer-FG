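; BP_Elevator is a moving platform that carries its Cube along a spline when either of two optional buttons is pressed.
; Each button's Pressed event plays the SplineMove timeline forward or in reverse, based on that button's DidInteract state.
; The timeline alpha maps to distance along the spline, with play rate derived from TimeToComplete.
; An optional pickup attaches to the Cube on BeginPlay.
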(event `self.ReceiveBeginPlay`
  ; Button 1
  (bind _button (`self.Button`)
    (:`then`
      (add `/Game/MovingBPs/BP_InteractableBase.Pressed` _button (delegate `Pressed_Event`)))
    (:`else`
      _))
  ; Button 2
  (bind _button2 (`self.Button2`)
    (:`then`
      (add `/Game/MovingBPs/BP_InteractableBase.Pressed` _button2 (delegate `Pressed_Event_0`)))
    (:`else`
      _))
  (bind _pickuptoattach (`self.PickupToAttach`)
    (:`then`
      (`self.K2_AttachToComponent` _pickuptoattach (`self.Cube`) "None" "SnapToTarget" "SnapToTarget" "KeepWorld" true))
    (:`else`)))

(event `Pressed_Event`
  ; Button 1
  (if (`/Game/MovingBPs/BP_InteractableBase.DidInteract` (`self.Button`))
    (`self.Move`)
    (else
      (`self.Reverse`))))

(event `Pressed_Event_0`
  ; Button 2
  (if (`/Game/MovingBPs/BP_InteractableBase.DidInteract` (stale `self.ReceiveBeginPlay` _button2))
    (`self.Move`)
    (else
      (`self.Reverse`))))

(event `Move`
  (bind _spline (`self.Spline`))
  ; Moving actor
  (`TimelineComponent.SetPlayRate` (`self.SplineMove`) (/ 1.0 (`self.TimeToComplete`)))
  (bind (_direction _move) (`Timeline|SplineMove` :!label _label)
    (:`Update`
      (`SceneComponent.K2_SetWorldLocation` (`self.Cube`) (`SplineComponent.GetLocationAtDistanceAlongSpline` _spline (`KismetMathLibrary.Lerp` 0.0 (`SplineComponent.GetSplineLength` _spline) _move) "World") false false))))

(event `Reverse`
  ; Moving actor
  (`TimelineComponent.SetPlayRate` (`self.SplineMove`) (/ 1.0 (`self.TimeToComplete`)))
  (goto _label :!via `Reverse`))

(fn `UserConstructionScript`)