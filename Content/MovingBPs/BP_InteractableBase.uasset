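; BP_InteractableBase is a base interactable button that toggles between pressed and released states.
; Interact flips the DidInteract RepNotify variable, so the state replicates.
; Its OnRep moves the Button component to a pressed offset or back to rest, then calls the Pressed dispatcher on either change.
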(event `Interact`
  (if (`self.DidInteract`)
    (set `self.DidInteract` false)
    (else
      (set `self.DidInteract` true))))

(event `PressButton`
  (`SceneComponent.K2_SetRelativeLocation` (`self.Button`) (0.0 -20.0 0.0) false false))

(event `DeactivateButton`
  (`SceneComponent.K2_SetRelativeLocation` (`self.Button`) (0.0 0.0 0.0) false false))

(fn `OnRep_DidInteract`
  (if (`self.DidInteract`)
    (`self.PressButton`)
    (else
      (`self.DeactivateButton`)))
  (`self.Pressed`))

(fn `UserConstructionScript`)